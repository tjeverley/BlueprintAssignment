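; BP_Door is a hinged door that the player swings open with the E key.
; Overlap events on its Box set CanOpen while a BP_FirstPersonDan is inside.
; Pressing E in range plays the DoorOpening timeline, which lerps the Door's yaw to a quarter turn.
; Pressing E out of range reverses the timeline, so the door only closes once the player has left the box.
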(event OnComponentBeginOverlap(Box)
  (params (OverlappedComponent :type Primitive%20Component%20Object%20Reference) (OtherActor :type Actor%20Object%20Reference) (OtherComp :type Primitive%20Component%20Object%20Reference) (OtherBodyIndex :type Integer) (bFromSweep :type Boolean) (SweepResult :type Hit%20Result%20Structure%20%28by%20ref%29))
  ;[0.15 0.15 0.15 0.5] Checks to see if the player can open doors
  (Utilities|Casting|CastToBP_FirstPersonDan OtherActor)
  (Variables|Default|SetbCanOpen true))

(event OnComponentEndOverlap(Box)
  (params (OverlappedComponent :type Primitive%20Component%20Object%20Reference) (OtherActor :type Actor%20Object%20Reference) (OtherComp :type Primitive%20Component%20Object%20Reference) (OtherBodyIndex :type Integer))
  ;[0.15 0.15 0.15 0.5] Checks to see if the player can open doors
  (Utilities|Casting|CastToBP_FirstPersonDan OtherActor)
  (Variables|Default|SetbCanOpen false))

(event EventBeginPlay)

(event Collision|EventActorBeginOverlap
  (params (OtherActor :type Actor%20Object%20Reference)))

(event EventTick
  (params (DeltaSeconds :type Float%20%28single-precision%29)))

(event Input|KeyboardEvents|E
  (params (Key :type Key%20Structure))
  ;[0.15 0.15 0.15 0.5] Interact with Door
  (:Pressed
    (if (Variables|Default|GetbCanOpen)
      (bind _dooe (Timeline|Door%20Opening Play)
        (:Update
          (Transformation|SetRelativeRotation (Variables|Default|GetDoor) (Math|Rotator|MakeRotator 0.0 0.0 (Math|Float|Lerp 0.0 9e+01 _dooe)) false false)))
      (else
        (Timeline|Door%20Opening Reverse)))))

(fn ConstructionScript)