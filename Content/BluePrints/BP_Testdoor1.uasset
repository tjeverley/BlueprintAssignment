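; BP_Testdoor1 is a test door that the first-person player (BP_FirstPersonDan) can swing open and closed.
; A box overlap caches the player and sets Inside, but end overlap clears CanOpen instead, so Inside stays true.
; Tick polls the player's PressCheck, flip-flopping the DoorOpening timeline between play and reverse on every frame it is true.
; The timeline scales the door's relative yaw up to 90 degrees.
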(event OnComponentBeginOverlap(Box)
  (params (OverlappedComponent :type Primitive%20Component%20Object%20Reference) (OtherActor :type Actor%20Object%20Reference) (OtherComp :type Primitive%20Component%20Object%20Reference) (OtherBodyIndex :type Integer) (bFromSweep :type Boolean) (SweepResult :type Hit%20Result%20Structure%20%28by%20ref%29))
  ;[0.15 0.15 0.15 0.5] Checks to see if the player can open doors
  (bind _asbp_first_person_b (Utilities|Casting|CastToBP_FirstPersonDan OtherActor))
  (Variables|Default|SetInside? true))

(event OnComponentEndOverlap(Box)
  (params (OverlappedComponent :type Primitive%20Component%20Object%20Reference) (OtherActor :type Actor%20Object%20Reference) (OtherComp :type Primitive%20Component%20Object%20Reference) (OtherBodyIndex :type Integer))
  ;[0.15 0.15 0.15 0.5] Checks to see if the player can open doors
  (Utilities|Casting|CastToBP_FirstPersonDan OtherActor)
  (Variables|Default|SetbCanOpen false))

(event EventBeginPlay)

(event Collision|EventActorBeginOverlap
  (params (OtherActor :type Actor%20Object%20Reference)))

(event EventTick
  (params (DeltaSeconds :type Float%20%28single-precision%29))
  (if (Variables|Default|GetInside?)
    ;[0.15 0.15 0.15 0.5] Checks to see if the player can open doors
    (if (Variables|/Game/FirstPerson/Blueprints/BP_FirstPersonDan.BP_FirstPersonDan_C|GetbPressCheck (stale OnComponentBeginOverlap(Box) _asbp_first_person_b))
      (Utilities|FlowControl|FlipFlop
        (:A
          (bind _dooe (Timeline|Door%20Opening Play)
            (:Update
              (Transformation|SetRelativeRotation (Variables|Default|GetDoor) (Math|Rotator|MakeRotator 0.0 0.0 (* _dooe 9e+01)) false false))))
        (:B
          (Timeline|Door%20Opening Reverse))))))

(fn ConstructionScript)