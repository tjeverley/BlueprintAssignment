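; BP_Pickable_object is an item actor that registers itself as available for pickup by the first-person player character.
; A Sphere overlap casts player pawn 0 to BP_FirstPersonDan and adds the item to its PickUpInRange array, without checking the overlapping actor.
; End overlap removes it through the same cast result.
; BeginPlay looks up a data table row by ID, but the result is unused.
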(event OnComponentBeginOverlap(Sphere)
  (params (OverlappedComponent :type Primitive%20Component%20Object%20Reference) (OtherActor :type Actor%20Object%20Reference) (OtherComp :type Primitive%20Component%20Object%20Reference) (OtherBodyIndex :type Integer) (bFromSweep :type Boolean) (SweepResult :type Hit%20Result%20Structure%20%28by%20ref%29))
  (bind _asbp_first_person_b (Utilities|Casting|CastToBP_FirstPersonDan (Game|Player|GetPlayerPawn 0)))
  (Utilities|Array|Add (Variables|/Game/FirstPerson/Blueprints/BP_FirstPersonDan.BP_FirstPersonDan_C|GetPickUpInRange _asbp_first_person_b) self))

(event OnComponentEndOverlap(Sphere)
  (params (OverlappedComponent :type Primitive%20Component%20Object%20Reference) (OtherActor :type Actor%20Object%20Reference) (OtherComp :type Primitive%20Component%20Object%20Reference) (OtherBodyIndex :type Integer))
  (Utilities|Array|RemoveItem (Variables|/Game/FirstPerson/Blueprints/BP_FirstPersonDan.BP_FirstPersonDan_C|GetPickUpInRange (stale OnComponentBeginOverlap(Sphere) _asbp_first_person_b)) self))

(event EventBeginPlay
  (Utilities|GetDataTableRow 0 (Utilities|String|StringToName (Variables|Default|GetID))))

(event Collision|EventActorBeginOverlap
  (params (OtherActor :type Actor%20Object%20Reference)))

(event EventTick
  (params (DeltaSeconds :type Float%20%28single-precision%29)))

(fn ConstructionScript)