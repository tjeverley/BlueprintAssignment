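; BP_Key is a pickup key that the first-person player character collects by pressing the interact input while standing in its overlap area.
; Overlap begin and end on the Key component cache the BP_FirstPersonDan reference and toggle an InsideCheck flag.
; Tick polls that flag and the character's PressCheck, then sets Keytake on the character and destroys the key actor.
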(event OnComponentBeginOverlap(Key)
  (params (OverlappedComponent :type Primitive%20Component%20Object%20Reference) (OtherActor :type Actor%20Object%20Reference) (OtherComp :type Primitive%20Component%20Object%20Reference) (OtherBodyIndex :type Integer) (bFromSweep :type Boolean) (SweepResult :type Hit%20Result%20Structure%20%28by%20ref%29))
  (bind _asbp_first_person_b (Utilities|Casting|CastToBP_FirstPersonDan OtherActor))
  (Variables|Default|SetInside%20Check true))

(event OnComponentEndOverlap(Key)
  (params (OverlappedComponent :type Primitive%20Component%20Object%20Reference) (OtherActor :type Actor%20Object%20Reference) (OtherComp :type Primitive%20Component%20Object%20Reference) (OtherBodyIndex :type Integer))
  (Utilities|Casting|CastToBP_FirstPersonDan OtherActor)
  (Variables|Default|SetInside%20Check false))

(event EventBeginPlay)

(event Collision|EventActorBeginOverlap
  (params (OtherActor :type Actor%20Object%20Reference)))

(event EventTick
  (params (DeltaSeconds :type Float%20%28single-precision%29))
  (if (Variables|Default|GetInside%20Check)
    (if (Variables|/Game/FirstPerson/Blueprints/BP_FirstPersonDan.BP_FirstPersonDan_C|GetbPressCheck (stale OnComponentBeginOverlap(Key) _asbp_first_person_b))
      (Variables|/Game/FirstPerson/Blueprints/BP_FirstPersonDan.BP_FirstPersonDan_C|SetKeytake (stale OnComponentBeginOverlap(Key) _asbp_first_person_b) true)
      (Actor|DestroyActor))))

(fn ConstructionScript)