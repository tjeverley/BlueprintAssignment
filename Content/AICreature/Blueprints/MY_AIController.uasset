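; AI controller that runs the BT_AI behavior tree on BeginPlay and feeds it sight and hearing perception through the Blackboard.
; Each perception update goes to two handlers that filter by sense class.
; Sight sets bCanSeePlayer only for BP_FirstPersonLiam actors.
; Hearing accepts any source, writing the stimulus location to TargetLocation and the sensed state to bCanHearPlayer, with a debug print.
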(event OnTargetPerceptionUpdated(AIPerception)
  (params (Actor :type Actor%20Object%20Reference) (Stimulus :type AI%20Stimulus%20Structure))
  ;[0.15 0.1388 0 0.5] Sight perception for AI
  (CallFunction|HandleSightSense Actor Stimulus)
  (CallFunction|HandleSoundSense Stimulus))

(event EventBeginPlay
  ;[0 0.15 0.01062 0.5] Start game and run behaviour tree
  (AI|RunBehaviorTree "/Game/AICreature/Blueprints/BT_AI.BT_AI"))

(event EventTick
  (params (DeltaSeconds :type Float%20%28single-precision%29)))

(fn ConstructionScript)

(fn HandleSoundSense
  (params (Stimulus :type AI%20Stimulus%20Structure%20%28by%20ref%29))
  (bind (_age _expirationage _strength _stimuluslocation _receiverlocation _tag _bsuccessfullysensed) (Utilities|Struct|BreakAIStimulus Stimulus))
  ;[0.01278 0.15 0.01294 0.5] Sound Logic For AI Perception
  (bind _returnvalue (Class|AIPerceptionSystem|GetSenseClassforStimulus Stimulus))
  (if (== _returnvalue "/Script/AIModule.AISense_Hearing")
    (AI|Components|Blackboard|SetValueasVector (Variables|Default|GetBlackboard) (Utilities|Name|MakeLiteralName "TargetLocation") _stimuluslocation)
    (AI|Components|Blackboard|SetValueasBool (AI|GetBlackboard 0) (Utilities|Name|MakeLiteralName "bCanHearPlayer") _bsuccessfullysensed)
    (Development|PrintString "Heard")))

(fn HandleSightSense
  (params (Object :type Object%20Object%20Reference) (AIStimulus :type AI%20Stimulus%20Structure))
  ;[0.00934 0.15 0.009297 0.5] Sight Logic For AI Perception
  (Utilities|Casting|CastToBP_FirstPersonLiam Object)
  (bind _returnvalue (Class|AIPerceptionSystem|GetSenseClassforStimulus AIStimulus))
  (if (== _returnvalue "/Script/AIModule.AISense_Sight")
    (AI|Components|Blackboard|SetValueasBool (AI|GetBlackboard 0) (Utilities|Name|MakeLiteralName "bCanSeePlayer") (.bSuccessfullySensed (Utilities|Struct|BreakAIStimulus AIStimulus)))))