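; BP_CommsUnit is a repairable comms unit that starts broken and lights up once the player repairs it.
; The InteractionDetector overlap events toggle CanInteract and cache the first BP_FirstPersonTom as PlayerRef; once cached, any actor's overlap toggles the flag.
; Tick polls the player's Activate flag while interaction is allowed to set Repaired, and sets the PointLight intensity from that state every frame.
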(event OnComponentBeginOverlap(InteractionDetector)
  (params (OverlappedComponent :type Primitive%20Component%20Object%20Reference) (OtherActor :type Actor%20Object%20Reference) (OtherComp :type Primitive%20Component%20Object%20Reference) (OtherBodyIndex :type Integer) (bFromSweep :type Boolean) (SweepResult :type Hit%20Result%20Structure%20%28by%20ref%29))
  ;[0.15 0.15 0.15 0.5] Interaction Detection
  (Utilities|IsValid (Variables|Default|GetPlayerRef)
    (:Is%20Valid
      _)
    (:Is%20Not%20Valid
      (bind _asbp_first_person_a (Utilities|Casting|CastToBP_FirstPersonTom OtherActor))
      (Variables|Default|SetPlayerRef _asbp_first_person_a)))
  (Variables|Default|SetbCanInteract true))

(event OnComponentEndOverlap(InteractionDetector)
  (params (OverlappedComponent :type Primitive%20Component%20Object%20Reference) (OtherActor :type Actor%20Object%20Reference) (OtherComp :type Primitive%20Component%20Object%20Reference) (OtherBodyIndex :type Integer))
  ;[0.15 0.15 0.15 0.5] Interaction Detection
  (Utilities|IsValid (Variables|Default|GetPlayerRef)
    (:Is%20Valid
      _)
    (:Is%20Not%20Valid
      (bind _asbp_first_person_a (Utilities|Casting|CastToBP_FirstPersonTom OtherActor))
      (Variables|Default|SetPlayerRef _asbp_first_person_a)))
  (Variables|Default|SetbCanInteract false))

(event EventBeginPlay
  ;[0.15 0.15 0.15 0.5] Set repaired to false by default
  (Variables|Default|SetbRepaired false))

(event EventTick
  (params (DeltaSeconds :type Float%20%28single-precision%29))
  (bind _playerref (Variables|Default|GetPlayerRef))
  (Utilities|FlowControl|Sequence
    (:then_0
      ;[0.15 0.15 0.15 0.5] Check for Player Ref
      (Utilities|IsValid _playerref
        (:Is%20Valid
          _)
        (:Is%20Not%20Valid
          (Utilities|Casting|CastToBP_FirstPersonTom _playerref)))
      ;[0.15 0.15 0.15 0.5] Repair Comms
      (if (and (Variables|/Game/FirstPerson/Blueprints/BP_FirstPersonTom.BP_FirstPersonTom_C|GetbActivate _playerref) (Variables|Default|GetbCanInteract))
        (if (not (Variables|Default|GetbRepaired))
          (Variables|Default|SetbRepaired true))))
    (:then_1
      ;[0.15 0.15 0.15 0.5] Check for repaired status
      (if (Variables|Default|GetbRepaired)
        (Rendering|Components|Light|SetIntensity (Variables|Default|GetPointLight) 1.5e+05)
        (else
          (Rendering|Components|Light|SetIntensity (Variables|Default|GetPointLight) 0.0))))))

(fn ConstructionScript)